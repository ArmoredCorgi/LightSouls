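; Enemy Blueprint that patrols four waypoints in a loop and chases the player once PawnSensing spots them.
; Chained AIMoveTo calls drive the patrol, while the chase re-issues its move after each success or failure.
; Capsule overlaps during the player's melee attack cost health behind a short hit cooldown, destroying the enemy at zero.
; Lockon toggles a targeting sphere, and an unused random-patrol routine is also present.
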(event `self.ReceiveBeginPlay`
  (`self.Patrol`))

(event `self.ReceiveTick`
  (params (DeltaSeconds :type "Float (single-precision)"))
  (`KismetSystemLibrary.Delay` 2.0)
  (if (not (`self.IsMoving`))
    (set `self.IsMoving` true)
    (`self.Patrol`)
    (set `self.IsMoving` false)))

(event `self.PawnSensing.OnSeePawn`
  (params (Pawn :type "Pawn Object Reference"))
  (`self.FollowPlayer` Pawn))

(event `Patrol`
  (`self.WaypointPatrol`)
  (`self.Patrol`))

(event `/Game/Blueprints/LockOnSystem.Lock On`
  (`/Engine/EditorBlueprintResources/StandardMacros.FlipFlop`
    (:`A`
      (`SceneComponent.SetVisibility` (`self.LockOnSphere`) true false))
    (:`B`
      (`SceneComponent.SetVisibility` (`self.LockOnSphere`) false false))))

(event `self.CapsuleComponent.OnComponentBeginOverlap`
  (params (OverlappedComponent :type "PrimitiveComponent Object Reference") (OtherActor :type "Actor Object Reference") (OtherComp :type "PrimitiveComponent Object Reference") (OtherBodyIndex :type Integer) (bFromSweep :type Boolean) (SweepResult :type "HitResult Structure (by ref)"))
  (`self.CheckCollisionForTakingDamage`))

(fn `DistanceToPlayer`
  (set `self.DistFromEnemyToPlayer` (`self.GetDistanceTo` (`GameplayStatics.GetPlayerPawn` 0)))
  (set `self.CanBeTargeted` true)
  (return))

(fn `TakeDamage`
  (returns (IsDead :type Boolean))
  (`GameplayStatics.SpawnEmitterAtLocation` "/Game/InfinityBladeEffects/Effects/FX_Combat_Base/Impact/P_Impact_Enemy_Strong.P_Impact_Enemy_Strong" (`self.K2_GetActorLocation`))
  (bind _output_get (set `self.Health` (- (`self.Health`) 50.0)))
  (return (<= _output_get 0.0)))

(fn `UserConstructionScript`)