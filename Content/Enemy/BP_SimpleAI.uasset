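; BP_SimpleAI is an enemy that takes melee damage from the player's one-handed sword and is destroyed when its health runs out.
; A capsule overlap with Weapon_Sword_1H calls TakeDamage only while BP_Player is attacking and the enemy is hittable.
; TakeDamage spawns an impact emitter, subtracts fixed damage and reports death.
; A surviving enemy blocks further melee hits for a short delay, and the graphs contain no movement or decision logic.
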(event `self.CapsuleComponent.OnComponentBeginOverlap`
  (params (OverlappedComponent :type "PrimitiveComponent Object Reference") (OtherActor :type "Actor Object Reference") (OtherComp :type "PrimitiveComponent Object Reference") (OtherBodyIndex :type Integer) (bFromSweep :type Boolean) (SweepResult :type "HitResult Structure (by ref)"))
  (cast `/Game/Player/Weapon_Sword_1H` OtherActor)
  (bind _asbp_player (cast `/Game/Player/BP_Player` (`GameplayStatics.GetPlayerCharacter` 0)))
  (if (`/Game/Player/BP_Player.IsAttacking1H` _asbp_player)
    (if (`self.CanBeHitWithMelee`)
      (bind _isdead (`self.TakeDamage`))
      (if _isdead
        (`self.K2_DestroyActor`)
        (else
          (set `self.CanBeHitWithMelee` false)
          (`KismetSystemLibrary.Delay` 1.0)
          (set `self.CanBeHitWithMelee` true))))))

(fn `TakeDamage`
  (returns (IsDead :type Boolean))
  (`GameplayStatics.SpawnEmitterAtLocation` "/Game/Imports/InfinityBladeEffects/Effects/FX_Monsters/FX_Monster_Ausar/P_AU_Shieldslam_Impact.P_AU_Shieldslam_Impact" (`self.K2_GetActorLocation`))
  (bind _output_get (set `self.Health` (- (`self.Health`) 50.0)))
  (return (<= _output_get 0.0)))

(fn `UserConstructionScript`)