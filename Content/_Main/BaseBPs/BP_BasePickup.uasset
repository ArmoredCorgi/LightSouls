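; BP_BasePickup is a base pickup actor whose Item component simulates physics from BeginPlay.
; On the server, a SphereCollision overlap by an actor tagged Player passes the pickup to that actor through SetPickupInfoMessage.
; A DisablePhysics event stops the simulation and turns off collision on both the item and the sphere.
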(event `self.ReceiveBeginPlay`
  (`PrimitiveComponent.SetSimulatePhysics` (`self.Item`) true))

(event `/Game/_Main/Interfaces/BPI_Pickups.DisablePhysics`
  (`PrimitiveComponent.SetSimulatePhysics` (`self.Item`) false)
  (`PrimitiveComponent.SetCollisionEnabled` (`self.Item`) "NoCollision")
  (`PrimitiveComponent.SetCollisionEnabled` (`self.SphereCollision`) "NoCollision"))

(event `self.SphereCollision.OnComponentBeginOverlap`
  (params (OverlappedComponent :type "PrimitiveComponent Object Reference") (OtherActor :type "Actor Object Reference") (OtherComp :type "PrimitiveComponent Object Reference") (OtherBodyIndex :type Integer) (bFromSweep :type Boolean) (SweepResult :type "HitResult Structure (by ref)"))
  (`/Engine/EditorBlueprintResources/ActorMacros.Switch Has Authority`
    (:`Authority`
      (if (`self.ActorHasTag` OtherActor "Player")
        (message `/Game/_Main/Interfaces/BPI_PlayerChar.SetPickupInfo` OtherActor self)))))

(fn `UserConstructionScript`)