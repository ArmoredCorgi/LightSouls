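; Troll enemy Blueprint whose heavy and charge attacks damage and knock back the player, building on inherited combat functions.
; In combat, ChasePlayer picks an attack by target distance, waits, then uses AI MoveTo to close in and attack, clearing the target on failure.
; On authority, Heavy and Special attacks run identical forward sphere overlaps that damage hit pawns and launch Player-tagged characters away with upward bias.
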(event `/Game/_Main/Interfaces/BPI_EnemyAI.DoSphereOverlap`
  (`/Engine/EditorBlueprintResources/ActorMacros.Switch Has Authority`
    (:`Authority`
      (switch `/Game/_Main/Enemies/E_AI_AttackTypes` (`self.f_GetAttackType`)
        (:`NewEnumerator1`
          (`self.f_HeavyAttackWithKnockback`))
        (:`NewEnumerator3`
          (`self.f_ChargeAttackWithKnockback`))))))

(event `/Game/_Main/Interfaces/BPI_EnemyAI.ChasePlayer`
  (if (`self.f_GetCombatState`)
    (bind _length (`self.f_ChooseAttack` (`self.GetDistanceTo` self (`self.f_GetPlayerTarget`))))
    (`KismetSystemLibrary.Delay` (+ _length 0.5))
    (`|AIMoveTo` self (0.0 0.0 0.0) (`self.f_GetPlayerTarget`) 150.0 true
      (:`OnSuccess`
        (`/Game/_Main/Interfaces/BPI_EnemyAI.ChooseAttackType`))
      (:`OnFail`
        (`/Game/_Main/Interfaces/BPI_EnemyAI.ClearTarget`)))))

(fn `f_ChargeAttackWithKnockback`
  (bind _outactors (`KismetSystemLibrary.SphereOverlapActors` (+ (`self.K2_GetActorLocation`) (* (`self.GetActorForwardVector`) 200.0)) 100.0 (`|MakeArray` "ObjectTypeQuery3" :!type "EObjectTypeQuery Enum") null (`|MakeArray` self :!type "Actor Object Reference")))
  (for _array_element _outactors
    (`self.f_DamagePlayer` _array_element)
    (`self.f_KnockbackPlayer` _array_element)))

(fn `f_HeavyAttackWithKnockback`
  (bind _outactors (`KismetSystemLibrary.SphereOverlapActors` (+ (`self.K2_GetActorLocation`) (* (`self.GetActorForwardVector`) 200.0)) 100.0 (`|MakeArray` "ObjectTypeQuery3" :!type "EObjectTypeQuery Enum") null (`|MakeArray` self :!type "Actor Object Reference")))
  (for _array_element _outactors
    (`self.f_DamagePlayer` _array_element)
    (`self.f_KnockbackPlayer` _array_element)))

(fn `f_KnockbackPlayer`
  (params (Player :type "Actor Object Reference"))
  (bind _ascharacter (cast `Character` Player :!pure true))
  (bind (_returnvalue_x _returnvalue_y _returnvalue_z) (`KismetMathLibrary.BreakVector` (`KismetMathLibrary.GetDirectionUnitVector` (`self.K2_GetActorLocation`) (`self.K2_GetActorLocation` _ascharacter))))
  (if (`self.ActorHasTag` Player "Player")
    (`self.LaunchCharacter` _ascharacter (* (`KismetMathLibrary.MakeVector` _returnvalue_x _returnvalue_y (+ _returnvalue_z 1.0)) 600.0) false false)))

(fn `UserConstructionScript`
  (`parent.UserConstructionScript`))