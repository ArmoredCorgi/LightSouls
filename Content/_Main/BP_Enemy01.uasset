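; Melee-target enemy that patrols four waypoints in a loop and chases the player once PawnSensing spots them.
; Chasing repeats AIMoveTo after each success or failure, while Tick restarts idle patrols and turns the health bar toward the camera.
; One-handed sword overlaps deal damage mid-attack with a short hit cooldown, spawning impact particles and screen-projected damage numbers before destruction at zero health.
; Lockon toggles a target sphere's visibility.
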(event `self.ReceiveBeginPlay`
  (`|ExecutionSequence`
    (:`then_0`
      (`self.SetupHealthBar`)
      (`self.SetupDamageNumber`))
    (:`then_1`
      (`self.Patrol`))))

(event `self.ReceiveTick`
  (params (DeltaSeconds :type "Float (single-precision)"))
  (`|ExecutionSequence`
    (:`then_0`
      (`self.RotateHealthBarToPlayer`))
    (:`then_1`
      (`self.StartPatrollingIfNotMoving`))))

(event `self.PawnSensing.OnSeePawn`
  (params (Pawn :type "Pawn Object Reference"))
  (`self.FollowPlayer` Pawn))

(event `Patrol`
  (`self.WaypointPatrol`)
  (`self.Patrol`))

(event `/Game/Blueprints/BPI_LockOnSystem.Lock On`
  (`/Engine/EditorBlueprintResources/StandardMacros.FlipFlop`
    (:`A`
      (`SceneComponent.SetVisibility` (`self.LockOnSphere`) true false))
    (:`B`
      (`SceneComponent.SetVisibility` (`self.LockOnSphere`) false false))))

(event `self.CapsuleComponent.OnComponentBeginOverlap`
  (params (OverlappedComponent :type "PrimitiveComponent Object Reference") (OtherActor :type "Actor Object Reference") (OtherComp :type "PrimitiveComponent Object Reference") (OtherBodyIndex :type Integer) (bFromSweep :type Boolean) (SweepResult :type "HitResult Structure (by ref)"))
  (bind _asweapon_sword_1h (cast `/Game/Blueprints/Weapon_Sword_1H` OtherActor))
  (`self.CheckCollisionAndTakeDamage` _asweapon_sword_1h))

(fn `DistanceToPlayer`
  (set `self.DistFromEnemyToPlayer` (`self.GetDistanceTo` (`GameplayStatics.GetPlayerPawn` 0)))
  (set `self.CanBeTargeted` true)
  (return))

(fn `SpawnDamageText`
  (params (SpawnLocation :type "Vector Structure") (DamageAmount :type "Float (double-precision)"))
  (bind _returnvalue (`|CreateWidget` "/Game/Blueprints/WBP_DamageNumberPopup.WBP_DamageNumberPopup_C" null DamageAmount (`GameplayStatics.ProjectWorldToScreen` (`GameplayStatics.GetPlayerController` 0) SpawnLocation true)))
  (`UserWidget.AddToViewport` _returnvalue 0))

(fn `TakeDamage`
  (params (Amount :type "Float (double-precision)"))
  (returns (IsDead :type Boolean))
  (`self.SpawnDamageText` (`SceneComponent.K2_GetComponentLocation` (`self.CapsuleComponent`)) Amount)
  (`GameplayStatics.SpawnEmitterAtLocation` "/Game/InfinityBladeEffects/Effects/FX_Combat_Base/Impact/P_Impact_Enemy_Strong.P_Impact_Enemy_Strong" (`self.K2_GetActorLocation`))
  (bind _output_get (set `self.CurrentHealth` (- (`self.CurrentHealth`) Amount)))
  (`/Game/Blueprints/WBP_EnemyHealthBar.UpdateHealth` (`self.EnemyHealthBarWidget`) _output_get)
  (return (<= _output_get 0.0)))

(fn `UserConstructionScript`)