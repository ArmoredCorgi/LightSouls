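; Interactable actor that notifies players when they enter or leave its sphere collision so they can set interaction info.
; On the server only, overlap begin and end events call SetInteractInfoMessage on actors tagged "Player", passing itself and the overlap state.
; GetMessageText and GetInteractType expose its message text and interaction type.
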(event `self.SphereCollision.OnComponentBeginOverlap`
  (params (OverlappedComponent :type "PrimitiveComponent Object Reference") (OtherActor :type "Actor Object Reference") (OtherComp :type "PrimitiveComponent Object Reference") (OtherBodyIndex :type Integer) (bFromSweep :type Boolean) (SweepResult :type "HitResult Structure (by ref)"))
  (`/Engine/EditorBlueprintResources/ActorMacros.Switch Has Authority`
    (:`Authority`
      (if (`self.ActorHasTag` OtherActor "Player")
        (message `/Game/_Main/Player/INT_PlayerCharacter.SetInteractInfo` OtherActor self true)))))

(event `self.SphereCollision.OnComponentEndOverlap`
  (params (OverlappedComponent :type "PrimitiveComponent Object Reference") (OtherActor :type "Actor Object Reference") (OtherComp :type "PrimitiveComponent Object Reference") (OtherBodyIndex :type Integer))
  (`/Engine/EditorBlueprintResources/ActorMacros.Switch Has Authority`
    (:`Authority`
      (if (`self.ActorHasTag` OtherActor "Player")
        (message `/Game/_Main/Player/INT_PlayerCharacter.SetInteractInfo` OtherActor self false)))))

(fn `GetInteractType`
  (returns (InteractType :type "/Game/_Main/Interactables/E_InteractType Enum"))
  (return (`self.InteractType`)))

(fn `GetMessageText`
  (returns (Message :type Text))
  (return (`self.MessageText`)))

(fn `UserConstructionScript`)