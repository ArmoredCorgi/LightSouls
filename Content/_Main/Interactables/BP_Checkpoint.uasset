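; BP_Checkpoint is an interactable rest point that resets the AI through GS_LightSouls when used.
; Its rest event calls ResetAI on the game state only if PlayerResting is false, then sets the flag so repeat calls do nothing.
; On the server, a Player-tagged actor leaving the sphere has its interact message updated to non-overlapping and clears the flag, allowing another reset.
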(event `/Game/_Main/Interfaces/INT_Interactable.RestAtCheckpoint`
  (if (not (`self.PlayerResting`))
    (bind _asgs_light_souls (cast `/Game/_Main/BaseBPs/GS_LightSouls` (`GameplayStatics.GetGameState`)))
    (`/Game/_Main/BaseBPs/GS_LightSouls.ResetAI` _asgs_light_souls)
    (set `self.PlayerResting` true)))

(event `self.SphereCollision.OnComponentEndOverlap`
  (params (OverlappedComponent :type "PrimitiveComponent Object Reference") (OtherActor :type "Actor Object Reference") (OtherComp :type "PrimitiveComponent Object Reference") (OtherBodyIndex :type Integer))
  (`/Engine/EditorBlueprintResources/ActorMacros.Switch Has Authority`
    (:`Authority`
      (if (`self.ActorHasTag` OtherActor "Player")
        (message `/Game/_Main/Player/INT_PlayerCharacter.SetInteractInfo` OtherActor self false)
        (set `self.PlayerResting` false)))))

(fn `UserConstructionScript`
  (`parent.UserConstructionScript`))