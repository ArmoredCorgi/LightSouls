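; Base NPC Blueprint that players can approach and interact with, exposing its Name through GetName.
; On the server, InteractCollider overlaps with actors tagged Player set that player's NPC text UI message, passing the NPC itself, and clear it on exit.
; The Interact event only prints the display name of the interacting PlayerCharacter.
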(event `/Game/_Main/Interactables/INT_Interact.Interact`
  (params (Interactor :type "Actor Object Reference"))
  (bind _asplayer_character (cast `/Game/_Main/Player/PlayerCharacter` Interactor))
  (`KismetSystemLibrary.PrintString` (`KismetSystemLibrary.GetDisplayName` _asplayer_character)))

(event `self.InteractCollider.OnComponentBeginOverlap`
  (params (OverlappedComponent :type "PrimitiveComponent Object Reference") (OtherActor :type "Actor Object Reference") (OtherComp :type "PrimitiveComponent Object Reference") (OtherBodyIndex :type Integer) (bFromSweep :type Boolean) (SweepResult :type "HitResult Structure (by ref)"))
  (`/Engine/EditorBlueprintResources/ActorMacros.Switch Has Authority`
    (:`Authority`
      (if (`self.ActorHasTag` OtherActor "Player")
        (message `/Game/_Main/Player/INT_PlayerCharacter.SetNPCTextUI` OtherActor self)))))

(event `self.InteractCollider.OnComponentEndOverlap`
  (params (OverlappedComponent :type "PrimitiveComponent Object Reference") (OtherActor :type "Actor Object Reference") (OtherComp :type "PrimitiveComponent Object Reference") (OtherBodyIndex :type Integer))
  (`/Engine/EditorBlueprintResources/ActorMacros.Switch Has Authority`
    (:`Authority`
      (if (`self.ActorHasTag` OtherActor "Player")
        (message `/Game/_Main/Player/INT_PlayerCharacter.ClearNPCTextUI` OtherActor)))))

(fn `GetName`
  (returns (Name :type String))
  (return (`self.Name`)))

(fn `UserConstructionScript`
  (`parent.UserConstructionScript`))