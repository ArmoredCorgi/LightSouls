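; Base pickup actor that drops into the world as a physics-simulated mesh and offers itself to players who come near.
; On the authority, sphere overlaps with actors tagged Player call SetPickupInfoMessage on that actor to flag the pickup as in or out of range.
; DisablePhysics turns off simulation and collision on both mesh and sphere.
; GetPickupType exposes the type stored in PickupInfo.
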(event `self.ReceiveBeginPlay`
  (`PrimitiveComponent.SetSimulatePhysics` (`self.StaticMesh`) true))

(event `/Game/_Main/Pickups/INT_Pickups.DisablePhysics`
  (bind _staticmesh (`self.StaticMesh`))
  (`PrimitiveComponent.SetSimulatePhysics` _staticmesh false)
  (`PrimitiveComponent.SetCollisionEnabled` _staticmesh "NoCollision")
  (`PrimitiveComponent.SetCollisionEnabled` (`self.SphereCollision`) "NoCollision"))

(event `self.SphereCollision.OnComponentBeginOverlap`
  (params (OverlappedComponent :type "PrimitiveComponent Object Reference") (OtherActor :type "Actor Object Reference") (OtherComp :type "PrimitiveComponent Object Reference") (OtherBodyIndex :type Integer) (bFromSweep :type Boolean) (SweepResult :type "HitResult Structure (by ref)"))
  (`/Engine/EditorBlueprintResources/ActorMacros.Switch Has Authority`
    (:`Authority`
      (if (`self.ActorHasTag` OtherActor "Player")
        (message `/Game/_Main/Player/INT_PlayerCharacter.SetPickupInfo` OtherActor self true)))))

(event `self.SphereCollision.OnComponentEndOverlap`
  (params (OverlappedComponent :type "PrimitiveComponent Object Reference") (OtherActor :type "Actor Object Reference") (OtherComp :type "PrimitiveComponent Object Reference") (OtherBodyIndex :type Integer))
  (`/Engine/EditorBlueprintResources/ActorMacros.Switch Has Authority`
    (:`Authority`
      (if (`self.ActorHasTag` OtherActor "Player")
        (message `/Game/_Main/Player/INT_PlayerCharacter.SetPickupInfo` OtherActor self false)))))

(fn `GetPickupType`
  (returns (PickupType :type "/Game/_Main/Pickups/E_PickupTypes Enum"))
  (return (`.PickupType_24_BFC02771423DA93201A4DEA5168568C5` (break `/Game/_Main/Pickups/S_PickupInfo` (`self.PickupInfo`)))))

(fn `UserConstructionScript`)