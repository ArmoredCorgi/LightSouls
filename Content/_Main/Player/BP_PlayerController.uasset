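; Player controller that owns the HUD, creating W_PlayerUI for the local player shortly after BeginPlay.
; Pickup messages, health, stamina and death events relay through Client events to update widgets on the owning client.
; The client health update ignores its HealthPercent input and always sends zero to the health bar.
; On death, it removes all widgets and shows W_Death.
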(event `self.ReceiveBeginPlay`
  (`KismetSystemLibrary.Delay` 0.2)
  (if (`self.IsLocalPlayerController`)
    (bind _returnvalue (`|CreateWidget` "/Game/_Main/Player/UI/W_PlayerUI.W_PlayerUI_C"))
    (bind _output_get (set `self.PlayerUI` _returnvalue))
    (`UserWidget.AddToViewport` _output_get 0)))

(event `/Game/_Main/Player/BPI_PlayerController.ShowPickupName`
  (params (State :type Boolean) (Name :type Text))
  (`self.Client_ShowPickupName` State Name))

(event `Client_ShowPickupName`
  (params (State :type Boolean) (Message :type Text))
  (`/Game/_Main/Player/UI/W_PlayerUI.PlayerMessage` (`self.PlayerUI`) State Message))

(event `/Game/_Main/Player/BPI_PlayerController.UpdatePlayerHealthUI`
  (params (HealthPercent :type "Float (single-precision)"))
  (`self.Client_UpdatePlayerHealthUI` HealthPercent))

(event `Client_UpdatePlayerHealthUI`
  (params (HealthPercent :type "Float (double-precision)"))
  (`/Game/_Main/Player/UI/W_PlayerUI.UpdateHealthBar` (`self.PlayerUI`) 0.0))

(event `/Game/_Main/Player/BPI_PlayerController.UpdateStaminaUI`
  (params (StaminaPercent :type "Float (single-precision)"))
  (`self.Client_UpdateStaminaUI` StaminaPercent))

(event `Client_UpdateStaminaUI`
  (params (StaminaPercent :type "Float (double-precision)"))
  (`/Game/_Main/Player/UI/W_PlayerUI.UpdateStaminaBar` (`self.PlayerUI`) StaminaPercent))

(event `/Game/_Main/Player/BPI_PlayerController.DeathScreenUI`
  (`self.Client_CreateDeathScreen`))

(event `Client_CreateDeathScreen`
  (`WidgetLayoutLibrary.RemoveAllWidgets`)
  (bind _returnvalue (`|CreateWidget` "/Game/_Main/Player/UI/W_Death.W_Death_C"))
  (`UserWidget.AddToViewport` _returnvalue 0))

(fn `UserConstructionScript`)