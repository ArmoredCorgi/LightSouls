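; Player lock-on system that targets the nearest living enemy and toggles the lock on request.
; FindTargets sphere-overlaps enemy pawns around the player, skips dead ones and picks the closest within range.
; ToggleCameraLock messages the player pawn and the target's widget, releasing the target on unlock.
; A looping timer drops the lock when horizontal distance exceeds the search radius.
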(event `Initialize`
  (bind _aspawn (cast `Pawn` (`self.GetOwner`)))
  (bind _output_get (set `self.PlayerPawn` _aspawn))
  (bind _asplayer_controller (cast `PlayerController` (`Pawn.GetController` _output_get)))
  (set `self.PlayerController` _asplayer_controller))

(event `LockOnTarget`
  (if (`self.CurrentlyLockedOn`)
    (`self.ToggleCameraLock` false)
    (else
      (`self.FindTargets`))))

(event `ClearLockOnTarget`
  (`self.ToggleCameraLock` false))

(event `FindTargets`
  (bind _outactors (`KismetSystemLibrary.SphereOverlapActors` (`Actor.K2_GetActorLocation` (`self.PlayerPawn`)) 1500.0 (`|MakeArray` "ObjectTypeQuery3" :!type "EObjectTypeQuery Enum") "/Game/_Main/Enemy/BP_EnemyBase.BP_EnemyBase_C"))
  (for _array_element _outactors
    (bind _isdead (message `/Game/_Main/Enemy/INT_EnemyAI.IsAIDead` _array_element))
    (if (not _isdead)
      (`KismetArrayLibrary.Array_AddUnique` (`self.PotentialTargets`) _array_element)))
  (for _array_element_2 (`self.PotentialTargets`)
    (bind _returnvalue (`Actor.GetDistanceTo` (`self.PlayerPawn`) _array_element_2))
    (if (< _returnvalue (`self.ClosestDist`))
      (set `self.ClosestDist` _returnvalue)
      (set `self.LockedTarget` _array_element_2)))
  (set `self.ClosestDist` 1500.0)
  (`KismetArrayLibrary.Array_Clear` (`self.PotentialTargets`))
  (`self.LockedTarget`
    (:`then`
      (set `self.CurrentlyLockedOn` true)
      (`self.ToggleCameraLock` true)
      (bind _returnvalue_2 (`KismetSystemLibrary.K2_SetTimerDelegate` (delegate `CheckTargetDist`) 0.5 true))
      (set `self.CheckDistHandle` _returnvalue_2))
    (:`else`)))

(event `ToggleCameraLock`
  (params (State :type Boolean))
  (bind _output_get (set `self.CurrentlyLockedOn` State))
  (`|ExecutionSequence`
    (:`then_0`
      (message `/Game/_Main/Player/INT_PlayerCharacter.LockOnToTarget` (`self.PlayerPawn`) _output_get (`self.LockedTarget`)))
    (:`then_1`
      (message `/Game/_Main/Enemy/INT_EnemyAI.ToggleTargetWidget` (`self.LockedTarget`) _output_get (`self.GetOwner`)))
    (:`then_2`
      (if (not _output_get)
        (set `self.LockedTarget` null)))))

(event `CheckTargetDist`
  (if (> (`Actor.GetHorizontalDistanceTo` (`self.PlayerPawn`) (`self.LockedTarget`)) 1500.0)
    (`self.ToggleCameraLock` false)
    (`KismetSystemLibrary.K2_ClearAndInvalidateTimerHandle` (`self.CheckDistHandle`))))