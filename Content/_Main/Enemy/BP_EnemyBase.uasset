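; Base enemy Character that roams around its spawn point until given a player target, then fights until the target is invalid or dead.
; Aggro optionally plays a distance-gated taunt, then loops AIMoveTo chasing and distance-based attack selection with random montages, facing the player on Tick.
; Montages and death play through multicast events; damage is looked up by current attack type.
; Zero health triggers death, with an empty death-animation function and delayed destroy.
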(event `Multi_PlayMontage`
  (params (InSkeletalMeshComponent :type "SkeletalMeshComponent Object Reference") (MontageToPlay :type "AnimMontage Object Reference") (StartingSection :type Name))
  (`|PlayMontage` InSkeletalMeshComponent MontageToPlay 1.0 0.0 StartingSection))

(event `self.ReceiveTick`
  (params (DeltaSeconds :type "Float (single-precision)"))
  ;[1 1 1] Tick
  (if (`self.IsInCombat`)
    (`self.PlayerTarget`
      (:`then`
        (`self.LookAtPlayer`))
      (:`else`))))

(event `self.ReceiveBeginPlay`
  ;[1 1 1] Begin Play
  (`|ExecutionSequence`
    (:`then_0`
      (set `self.StartingLocation` (`self.K2_GetActorLocation`)))
    (:`then_1`
      (`self.f_MovementState` "NewEnumerator1")
      (`KismetSystemLibrary.Delay` 1.0)
      (`self.SetRoaming`))))

(event `self.SetRoaming`
  ;[1 1 1] Random Roaming
  (if (and (not (`self.IsInCombat`)) (not (`self.IsRoaming`)))
    (`self.Move_RandomRoam`
      (:`then`
        (set `self.IsRoaming` true))
      (:`PointReached`
        (set `self.IsRoaming` false)
        (`KismetSystemLibrary.Delay` 4.0)
        (`self.SetRoaming`)))))

(event `self.SetPlayerTarget`
  (params (PlayerTarget :type "Actor Object Reference"))
  ;[1 1 1] Player Has Aggro
  (set `self.PlayerTarget` PlayerTarget)
  (set `self.IsInCombat` true)
  (`self.SetActorTickEnabled` true)
  (set `self.CombatStartLocation` (`self.K2_GetActorLocation`))
  (`self.f_MovementState` "NewEnumerator2")
  (`self.CheckForTaunt`))

(event `self.CheckForTaunt`
  (bind _output (`self.f_GetRandomMontage` (`self.TauntMontage`)))
  ;[1 1 1] Taunt Player On Aggro
  (`Controller.StopMovement` (`self.GetController`))
  (`self.Check_ShouldTaunt`
    (:`then`
      (`self.Multi_PlayMontage` (`self.Mesh`) _output)
      (bind _returnvalue (`AnimSequenceBase.GetPlayLength` _output))
      (`KismetSystemLibrary.Delay` _returnvalue))
    (:`else`
      _))
  (`self.ChasePlayer`))

(event `self.ChasePlayer`
  ;[1 1 1] Chase Player
  (if (`self.IsInCombat`)
    (`|AIMoveTo` self (0.0 0.0 0.0) (`self.PlayerTarget`) 150.0 true
      (:`OnSuccess`
        (`self.ChooseAttackType`))
      (:`OnFail`
        (`self.ClearTarget`)))))

(event `self.ClearTarget`
  (set `self.IsInCombat` false))

(event `self.ChooseAttackType`
  (bind _playertarget (`self.PlayerTarget`)
    (:`then`
      (bind _dead (message `/Game/_Main/Interfaces/BPI_PlayerChar.IsDead` _playertarget))
      (if _dead
        (`self.ClearTarget`)
        (else
          (bind _length (`self.f_ChooseAttack` (`self.GetDistanceTo` self (`self.PlayerTarget`))))
          (`KismetSystemLibrary.Delay` (+ _length 0.5))
          (`self.ChasePlayer`))))
    (:`else`
      (`self.ClearTarget`))))

(event `self.ReceiveAnyDamage`
  (params (Damage :type "Float (single-precision)") (DamageType :type "DamageType Object Reference") (InstigatedBy :type "Controller Object Reference") (DamageCauser :type "Actor Object Reference"))
  (bind _output_get (set `self.MaxHealth` (- (`self.MaxHealth`) Damage)))
  (if (<= _output_get 0.0)
    (`self.Death`)))

(event `self.Death`
  (bind _charactermovement (`self.CharacterMovement`))
  (if (not (`self.IsDead`))
    (set `self.IsDead` true)
    (`self.Multi_DeadAnim`)
    (`self.ClearTarget`)
    (`self.DetachFromControllerPendingDestroy`)
    (`CharacterMovementComponent.SetAvoidanceEnabled` _charactermovement false)
    (`CharacterMovementComponent.DisableMovement` _charactermovement)
    (`KismetSystemLibrary.Delay` 5.0)
    (`self.K2_DestroyActor`)))

(event `Multi_DeadAnim`
  (`PrimitiveComponent.SetCollisionProfileName` (`self.CapsuleComponent`) "Ragdoll" true)
  (`SkeletalMeshComponent.SetAnimationMode` (`self.Mesh`) "AnimationSingleNode")
  (`self.f_PlayDeathAnim`))

(fn `f_ApplyDamageToPlayer`
  (params (DamagedActor :type "Actor Object Reference"))
  (returns (DamageApplied :type "Float (double-precision)"))
  (if (`self.ActorHasTag` DamagedActor "Player")
    (bind _returnvalue (`GameplayStatics.ApplyDamage` DamagedActor (`self.f_GetDamage` (`self.AttackTypes`)) null self "/Script/Engine.DamageType"))
    (return _returnvalue)))

(fn `f_ChooseAttack`
  (params (DistanceToPlayer :type "Float (double-precision)"))
  (returns (Length :type "Float (double-precision)"))
  (bind _output (`self.f_GetRandomMontage` (`self.SpecialAttackMontages`)))
  (bind _output_2 (`self.f_GetRandomMontage` (`self.RangedAttackMontages`)))
  (bind _output_3 (`self.f_GetRandomMontage` (`self.LightAttackMontages`)))
  (bind _output_4 (`self.f_GetRandomMontage` (`self.HeavyAttackMontages`)))
  (if (<= DistanceToPlayer (`self.MeleeDistance`))
    (if (`self.f_Percentage` 70.0)
      (set `self.AttackTypes` "NewEnumerator0")
      (`self.Multi_PlayMontage` (`self.Mesh`) _output_3)
      (bind _returnvalue (`AnimSequenceBase.GetPlayLength` _output_3))
      (return _returnvalue)
      (else
        (set `self.AttackTypes` "NewEnumerator1")
        (`self.Multi_PlayMontage` (`self.Mesh`) _output_4)
        (bind _returnvalue_2 (`AnimSequenceBase.GetPlayLength` _output_4))
        (return _returnvalue_2)))
    (elif (<= DistanceToPlayer (`self.RangedDistance`))
      (set `self.AttackTypes` "NewEnumerator3")
      (`self.Multi_PlayMontage` (`self.Mesh`) _output)
      (bind _returnvalue_3 (`AnimSequenceBase.GetPlayLength` _output))
      (return _returnvalue_3)
      (else
        (set `self.AttackTypes` "NewEnumerator2")
        (`self.Multi_PlayMontage` (`self.Mesh`) _output_2)
        (bind _returnvalue_4 (`AnimSequenceBase.GetPlayLength` _output_2))
        (return _returnvalue_4)))))

(fn `f_GetAttackType`
  (returns (AttackTypes :type "/Game/_Main/Enemy/E_AI_AttackTypes Enum"))
  (return (`self.AttackTypes`)))

(fn `f_GetCombatState`
  (returns (IsInCombat :type Boolean))
  (return (`self.IsInCombat`)))

(fn `f_GetDamage`
  (params (AIAttackTypes :type "/Game/_Main/Enemy/E_AI_AttackTypes Enum" :default "NewEnumerator0"))
  (returns (Damage :type "Float (double-precision)"))
  (switch `/Game/_Main/Enemy/E_AI_AttackTypes` AIAttackTypes
    (:`NewEnumerator0`
      (return (`self.LightAttackDamage`)))
    (:`NewEnumerator1`
      (return (`self.HeavyAttackDamage`)))
    (:`NewEnumerator2`
      (return (`self.RangedAttackDamage`)))
    (:`NewEnumerator3`
      (return (`self.SpecialAttackDamage`)))))

(fn `f_GetPlayerTarget`
  (returns (PlayerTarget :type "Actor Object Reference"))
  (return (`self.PlayerTarget`)))

(fn `f_GetRandomMontage`
  (params (Montages :type "Array of AnimMontage Object Reference"))
  (returns (Output :type "AnimMontage Object Reference"))
  (return (`|GetArrayItem` Montages (`KismetMathLibrary.RandomIntegerInRange` 0 (- (`KismetArrayLibrary.Array_Length` Montages) 1)))))

(fn `f_MovementState`
  (params (MoveState :type "/Game/_Main/Enemy/E_AIMovementState Enum" :default "NewEnumerator0"))
  (bind _walkspeed (`self.WalkSpeed`))
  (set `CharacterMovementComponent.MaxWalkSpeed` (select `/Game/_Main/Enemy/E_AIMovementState` MoveState :`NewEnumerator1` _walkspeed :`NewEnumerator2` (* _walkspeed (`self.SpeedMultiplier`))) (`self.CharacterMovement`)))

(fn `f_Percentage`
  (params (Percent :type "Float (double-precision)"))
  (returns (Return :type Boolean))
  (return (select `bool` (== Percent 0.0) :`false` (<= (`KismetMathLibrary.RandomFloatInRange` 0.0 100.0) Percent))))

(fn `f_PlayDeathAnim`)

(fn `UserConstructionScript`
  (`parent.UserConstructionScript`))