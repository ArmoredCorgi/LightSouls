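; Boss enemy Blueprint that makes a checkpoint appear when the boss dies.
; Its Death event runs the parent death logic, waits briefly, then calls a Multi-prefixed spawn event.
; That event plays an ice shatter effect just below the referenced spawn-location actor, then spawns the Checkpoint class at that actor's transform after a short delay.
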(event `/Game/_Main/BP_CharacterBase.Death`
  (params (MurderingActor :type "Actor Object Reference"))
  (`parent.Death` MurderingActor)
  (`KismetSystemLibrary.Delay` 1.5)
  (`self.Multi_SpawnCheckpoint`))

(event `Multi_SpawnCheckpoint`
  (bind _returnvalue (`self.GetTransform` (`self.CheckpointSpawnLocation`)))
  (`GameplayStatics.SpawnEmitterAtLocation` "/Game/InfinityBladeEffects/Effects/FX_Skill_Aura/P_Aura_Ice_Shatter_01.P_Aura_Ice_Shatter_01" (`KismetMathLibrary.MakeVector` (.x (.location _returnvalue)) (.y (.location _returnvalue)) (- (.z (.location _returnvalue)) 149.899994)))
  (`KismetSystemLibrary.Delay` 0.2)
  (`|SpawnActorFromClass` "/Game/_Main/Interactables/Checkpoint.Checkpoint_C" _returnvalue "AdjustIfPossibleButAlwaysSpawn" "OverrideRootScale" null null))

(fn `UserConstructionScript`
  (`parent.UserConstructionScript`))