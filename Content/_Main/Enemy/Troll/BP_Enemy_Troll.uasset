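; Troll enemy Blueprint, a child of a base enemy, that chases the player and attacks with melee hits or vomit projectiles.
; While in combat it picks an attack by distance, waits, moves to the target, then chooses an attack type, clearing the target on failure.
; Authority-only melee uses forward sphere overlaps to apply damage, with heavy and charge attacks launching players back.
; Taking damage multicasts a sword-hit sound.
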(event `self.ReceiveAnyDamage`
  (params (Damage :type "Float (single-precision)") (DamageType :type "DamageType Object Reference") (InstigatedBy :type "Controller Object Reference") (DamageCauser :type "Actor Object Reference"))
  ;[1 1 1] Take Damage Override
  (`parent.ReceiveAnyDamage` Damage DamageType InstigatedBy DamageCauser)
  (`self.Multi_PlaySwordHit` "/Game/_Main/Player/SoundFX/SwordHit_Cue.SwordHit_Cue" (`self.K2_GetActorLocation` DamageCauser)))

(event `Multi_PlaySwordHit`
  (params (Sound :type "SoundBase Object Reference") (Location :type "Vector Structure"))
  ;[1 1 1] Take Damage Override
  (`GameplayStatics.PlaySoundAtLocation` Sound Location (struct) 1.0 1.0 0.0 null null null))

(event `/Game/_Main/Enemy/INT_EnemyAI.ChasePlayer`
  ;[1 1 1] Charge Attack and Chase Player
  (if (`self.GetCombatState`)
    (bind _length (`self.ChooseAttack` (`self.GetDistanceTo` self (`self.GetPlayerTarget`))))
    (`KismetSystemLibrary.Delay` (+ _length 0.5))
    (`|AIMoveTo` self (0.0 0.0 0.0) (`self.GetPlayerTarget`) 150.0 true
      (:`OnSuccess`
        (`/Game/_Main/Enemy/INT_EnemyAI.ChooseAttackType`))
      (:`OnFail`
        (`/Game/_Main/Enemy/INT_EnemyAI.ClearTarget`)))))

(event `/Game/_Main/Enemy/INT_EnemyAI.DoMeleeAttack`
  ;[1 1 1] Melee Attacks
  (`/Engine/EditorBlueprintResources/ActorMacros.Switch Has Authority`
    (:`Authority`
      (switch `/Game/_Main/Enemy/E_AI_AttackTypes` (`self.GetAttackType`)
        (:`NewEnumerator0`
          (`self.f_LightAttack`))
        (:`NewEnumerator1`
          (`self.f_HeavyAttackWithKnockback`))
        (:`NewEnumerator3`
          (`self.f_ChargeAttackWithKnockback`))))))

(event `/Game/_Main/Enemy/INT_EnemyAI.DoRangedAttack`
  ;[1 1 1] Ranged Attack (Vomit)
  (`|SpawnActorFromClass` "/Game/_Main/Enemy/Troll/Projectile_Vomit.Projectile_Vomit_C" (`SceneComponent.K2_GetComponentToWorld` (`self.VomitSpawn`)) "AlwaysSpawn" "OverrideRootScale" self (`self.RangedAttackDamage`) null))

(fn `f_ChargeAttackWithKnockback`
  (bind _outactors (`KismetSystemLibrary.SphereOverlapActors` (+ (`self.K2_GetActorLocation`) (* (`self.GetActorForwardVector`) 200.0)) 100.0 (`|MakeArray` "ObjectTypeQuery3" :!type "EObjectTypeQuery Enum") null (`|MakeArray` self :!type "Actor Object Reference")))
  (for _array_element _outactors
    (`self.ApplyDamageToPlayer` _array_element)
    (`self.f_KnockbackPlayer` _array_element)))

(fn `f_HeavyAttackWithKnockback`
  (bind _outactors (`KismetSystemLibrary.SphereOverlapActors` (+ (`self.K2_GetActorLocation`) (* (`self.GetActorForwardVector`) 200.0)) 100.0 (`|MakeArray` "ObjectTypeQuery3" :!type "EObjectTypeQuery Enum") null (`|MakeArray` self :!type "Actor Object Reference")))
  (for _array_element _outactors
    (`self.ApplyDamageToPlayer` _array_element)
    (`self.f_KnockbackPlayer` _array_element)))

(fn `f_KnockbackPlayer`
  (params (Player :type "Actor Object Reference"))
  (bind _ascharacter (cast `Character` Player :!pure true))
  (bind (_returnvalue_x _returnvalue_y _returnvalue_z) (`KismetMathLibrary.BreakVector` (`KismetMathLibrary.GetDirectionUnitVector` (`self.K2_GetActorLocation`) (`self.K2_GetActorLocation` _ascharacter))))
  (if (`self.ActorHasTag` Player "Player")
    (`self.LaunchCharacter` _ascharacter (* (`KismetMathLibrary.MakeVector` _returnvalue_x _returnvalue_y (+ _returnvalue_z 1.0)) 600.0) false false)))

(fn `f_LightAttack`
  (bind _outactors (`KismetSystemLibrary.SphereOverlapActors` (+ (`self.K2_GetActorLocation`) (* (`self.GetActorForwardVector`) 200.0)) 100.0 (`|MakeArray` "ObjectTypeQuery3" :!type "EObjectTypeQuery Enum") null (`|MakeArray` self :!type "Actor Object Reference")))
  (for _array_element _outactors
    (`self.ApplyDamageToPlayer` _array_element)))

(fn `PlayDeathAnim`
  (`SkeletalMeshComponent.PlayAnimation` (`self.Mesh`) "/Game/_Main/Enemy/Troll/Animation/ExoGame_Troll_Death_.ExoGame_Troll_Death_" false))

(fn `UserConstructionScript`
  (`parent.UserConstructionScript`))