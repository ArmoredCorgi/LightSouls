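; Replicated enemy projectile that damages the first overlapped actor tagged Player or Enemy and plays a hit effect.
; On the authority, any sphere overlap flags a hit and destroys the projectile, with damage applied only to tagged actors and credited to the owner.
; When destroyed after a hit, it spawns the hit emitter at its location through what appears to be a multicast event.
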(event `self.Sphere.OnComponentBeginOverlap`
  (params (OverlappedComponent :type "PrimitiveComponent Object Reference") (OtherActor :type "Actor Object Reference") (OtherComp :type "PrimitiveComponent Object Reference") (OtherBodyIndex :type Integer) (bFromSweep :type Boolean) (SweepResult :type "HitResult Structure (by ref)"))
  (`/Engine/EditorBlueprintResources/ActorMacros.Switch Has Authority`
    (:`Authority`
      (if (or (`self.ActorHasTag` OtherActor "Player") (`self.ActorHasTag` OtherActor "Enemy"))
        (set `self.IsHit` true)
        (`GameplayStatics.ApplyDamage` OtherActor (`self.Damage`) null (`self.GetOwner`) "/Script/Engine.DamageType")
        (`self.K2_DestroyActor`)
        (else
          (set `self.IsHit` true)
          (`self.K2_DestroyActor`))))))

(event `self.ReceiveDestroyed`
  (if (`self.IsHit`)
    (`self.Multi_SpawnFX` (`self.EmitterHit`) (`self.K2_GetActorLocation`))))

(event `Multi_SpawnFX`
  (params (EmitterTemplate :type "ParticleSystem Object Reference") (Location :type "Vector Structure"))
  (`GameplayStatics.SpawnEmitterAtLocation` EmitterTemplate Location))

(fn `UserConstructionScript`)