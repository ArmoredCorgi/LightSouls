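; BP_BaseItem is a world pickup item, apparently a base class, that players can interact with to collect.
; Its physics-simulated mesh pairs with a sphere trigger that, on authority only, sets or clears item UI text on overlapping Player-tagged actors.
; Interact calls Multi_AddToInventory, which adds one unit of its ItemInfo to the player's Inventory_Component.
; DisablePhysics switches off simulation and both collisions; the item never destroys itself here.
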(event `self.Sphere.OnComponentBeginOverlap`
  (params (OverlappedComponent :type "PrimitiveComponent Object Reference") (OtherActor :type "Actor Object Reference") (OtherComp :type "PrimitiveComponent Object Reference") (OtherBodyIndex :type Integer) (bFromSweep :type Boolean) (SweepResult :type "HitResult Structure (by ref)"))
  (`/Engine/EditorBlueprintResources/ActorMacros.Switch Has Authority`
    (:`Authority`
      (if (`self.ActorHasTag` OtherActor "Player")
        (message `/Game/_Main/Player/INT_PlayerCharacter.SetItemTextUI` OtherActor self)))))

(event `self.ReceiveBeginPlay`
  (`PrimitiveComponent.SetSimulatePhysics` (`self.StaticMesh`) true))

(event `/Game/_Main/Items/INT_Interact.DisablePhysics`
  (bind _staticmesh (`self.StaticMesh`))
  (`PrimitiveComponent.SetSimulatePhysics` _staticmesh false)
  (`PrimitiveComponent.SetCollisionEnabled` _staticmesh "NoCollision")
  (`PrimitiveComponent.SetCollisionEnabled` (`self.Sphere`) "NoCollision"))

(event `self.Sphere.OnComponentEndOverlap`
  (params (OverlappedComponent :type "PrimitiveComponent Object Reference") (OtherActor :type "Actor Object Reference") (OtherComp :type "PrimitiveComponent Object Reference") (OtherBodyIndex :type Integer))
  (`/Engine/EditorBlueprintResources/ActorMacros.Switch Has Authority`
    (:`Authority`
      (if (`self.ActorHasTag` OtherActor "Player")
        (message `/Game/_Main/Player/INT_PlayerCharacter.ClearItemTextUI` OtherActor)))))

(event `/Game/_Main/Items/INT_Interact.Interact`
  (params (Player :type "Actor Object Reference"))
  (`self.Multi_AddToInventory` Player (`self.ItemInfo`)))

(event `Multi_AddToInventory`
  (params (Target :type "Actor Object Reference") (ItemInfo :type "/Game/_Main/Items/S_ItemInfo Structure"))
  (`/Game/_Main/Items/Inventory_Component.AddToInventory` (`self.GetComponentByClass` Target "/Game/_Main/Items/Inventory_Component.Inventory_Component_C") (make `/Game/_Main/Items/S_SlotInfo` ItemInfo 1)))

(fn `GetInteractType`
  (returns (InteractType :type "/Game/_Main/Interactables/E_InteractType Enum"))
  (return "NewEnumerator1"))

(fn `UserConstructionScript`)